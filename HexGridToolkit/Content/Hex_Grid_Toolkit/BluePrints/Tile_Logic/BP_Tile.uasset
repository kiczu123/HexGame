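; BP_Tile is a hex grid tile actor that places itself from axial coordinates and shows whether it is in sight.
; Update, run on BeginPlay, converts Axial to a 3D location and adds a slight random tilt, then refreshes the field-of-view look.
; FovSet stores the OnSight flag, and FovUpdate sets the material's Color parameter by tile Type, darkened when out of sight.
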(event `self.ReceiveBeginPlay`
  (`self.Update`))

(event `Update`
  (bind (_location2d _location3d) (`/Game/Hex_Grid_Toolkit/BluePrints/Hex_Logic/BPFL_Hex_Logic.AxialToLocation` (`self.Axial`)))
  (`self.K2_SetActorTransform` (`KismetMathLibrary.MakeTransform` _location3d (`KismetMathLibrary.RotatorFromAxisAndAngle` (`KismetMathLibrary.RandomUnitVector`) 2.0)))
  (`self.FovUpdate`))

(event `FovSet`
  (params (OnSight :type Boolean))
  (set `self.OnSight` OnSight)
  (`self.FOVUpdate`))

(event `FovUpdate`
  (bind _returnvalue (select `/Game/Hex_Grid_Toolkit/BluePrints/Tile_Logic/E_TileType` (`self.Type`) :`NewEnumerator0` (struct :`R` 0.296875 :`G` 0.296875 :`B` 0.296875 :`A` 1.0) :`NewEnumerator5` (struct :`R` 0.05 :`G` 0.05 :`B` 0.05 :`A` 1.0) :`NewEnumerator8` (struct :`R` 1.0 :`A` 1.0) :!type "LinearColor Structure"))
  (`MeshComponent.SetVectorParameterValueOnMaterials` (`self.SM_Tile`) "Color" (`KismetMathLibrary.Conv_LinearColorToVector` (select `bool` (`self.OnSight`) :`false` (* _returnvalue 0.35) :`true` _returnvalue))))

(fn `UserConstructionScript`)