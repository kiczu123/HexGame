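; Hex-grid tile manager that generates an island world and stores its tile actors in a map keyed by axial coordinate.
; BeginPlay spawns the region manager, fills a hexagon with water, stamps random plains islands, randomizes tiles from neighbor types, then initializes regions.
; Tick debug-draws selection, hover, shape and path; flood fill, Dijkstra, A* and FOV demos are switched off.
; An unexecuted definitions graph documents the toolkit's coordinate systems and functions.
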(event `self.ReceiveBeginPlay`
  (bind _returnvalue (`|SpawnActorFromClass` "/Game/System/RegionMenager.RegionMenager_C" (`self.GetTransform`) "Undefined" "OverrideRootScale" null self null))
  (set `self.RegionMenager` _returnvalue)
  (`self.WorldGenerator`))

(event `self.ReceiveTick`
  (params (DeltaSeconds :type "Float (single-precision)"))
  (`|ExecutionSequence`
    (:`then_0`
      (if true
        (`/Game/Hex_Grid_Toolkit/Hex_Logic/BPFL_Hex_Logic.DebugDrawHex` (`self.HexSelected`) (struct :`G` 1.0 :`A` 1.0))
        (`/Game/Hex_Grid_Toolkit/Hex_Logic/BPFL_Hex_Logic.DebugDrawHex` (`self.HexHover`) (struct :`B` 1.0 :`A` 1.0))
        (`/Game/Hex_Grid_Toolkit/Hex_Logic/BPFL_Hex_Logic.DebugDrawShape` (`self.DisplayShape`) (struct :`R` 0.552002 :`G` 0.724938 :`B` 0.890625 :`A` 1.0) 0.0)
        (`/Game/Hex_Grid_Toolkit/Hex_Logic/BPFL_Hex_Logic.DebugDrawPath` (`self.DisplayPath`))))
    (:`then_1`
      (if false
        (`/Game/Hex_Grid_Toolkit/Hex_Logic/BPFL_Hex_Logic.DebugDrawDirections` (`self.HexSelected`) (`self.HexHover`))))
    (:`then_2`
      (if false
        (bind _shapeout (`/Game/Hex_Grid_Toolkit/Hex_Logic/BPFL_Hex_Logic.getShape` "NewEnumerator1" (struct) (make `IntPoint` 10 5)))
        (bind _axials (`/Game/Hex_Grid_Toolkit/Hex_Logic/BPFL_Hex_Logic.TransformArray` _shapeout (`self.HexHover`)))
        (`/Game/Hex_Grid_Toolkit/Hex_Logic/BPFL_Hex_Logic.DebugDrawShape` _axials (struct :`R` 1.0 :`G` 0.502577 :`A` 1.0) 0.0)))))

(event `HexSelectedUpdate`
  (bind _shape (`self.findTilesOfType` (`self.TileMap`) (`self.getTileType` (`self.HexSelected`))))
  (`|ExecutionSequence`
    (:`then_0`
      (if false
        (bind _shape_2 (`/Game/Hex_Grid_Toolkit/Hex_Logic/BPFL_Hex_Logic.FloodFill` _shape (`self.HexHover`)))
        (set `self.DisplayShape` _shape_2)))
    (:`then_1`
      (if false
        (bind _flowmap (`/Game/Hex_Grid_Toolkit/Hex_Logic/BPFL_Hex_Logic.Dijkstra` _shape (`self.HexSelected`)))
        (`/Game/Hex_Grid_Toolkit/Hex_Logic/BPFL_Hex_Logic.DebugDrawFlowMap` _flowmap 2.0)))))

(event `SetRegionView`
  (params (RegionView :type Boolean))
  (bind _values (`BlueprintMapLibrary.Map_Values` (`self.TileMap`)))
  (for _array_element _values
    (`/Game/Hex_Grid_Toolkit/Tile_Logic/BP_Tile.SetRegionView` _array_element RegionView)))

(event `HexHoverUpdate`
  (`|ExecutionSequence`
    (:`then_0`
      (if false
        (bind _path (`/Game/Hex_Grid_Toolkit/Hex_Logic/BPFL_Hex_Logic.PathFromFlowMap` (stale `HexSelectedUpdate` _flowmap) (`self.HexHover`)))
        (set `self.DisplayPath` _path)))
    (:`then_1`
      (if false
        (bind _path_2 (`/Game/Hex_Grid_Toolkit/Hex_Logic/BPFL_Hex_Logic.AStar` (stale `HexSelectedUpdate` _shape) (`self.HexSelected`) (`self.HexHover`)))
        (set `self.DisplayPath` _path_2)))
    (:`then_2`
      (if false
        (`self.setTileSight` (stale _onsight))
        (bind _shape (`self.findTilesOfType` (`self.TileMap`) "NewEnumerator8"))
        (bind _onsight (`/Game/Hex_Grid_Toolkit/Hex_Logic/BPFL_Hex_Logic.scanFov` (make `/Game/Hex_Grid_Toolkit/Hex_Logic/S_Scan_Fov` (`self.HexHover`) 12 0 _shape 0.0 6.0))) ; BETA STAGE
        (`self.setTileSight` _onsight true)))))

(fn `ClearLandmass`
  (locals (RandomizerPull :type "Array of /Game/Hex_Grid_Toolkit/Tile_Logic/E_TileType Enum"))
  (bind _outitem (`KismetArrayLibrary.Array_Random` (`local.RandomizerPull`)))
  (bind _keys (`BlueprintMapLibrary.Map_Keys` (`self.TileMap`)))
  (for _array_element _keys
    (bind _axials (`/Game/Hex_Grid_Toolkit/Hex_Logic/BPFL_Hex_Logic.getAllAdjacentsCW` _array_element))
    (for _array_element_2 _axials
      (switch `/Game/Hex_Grid_Toolkit/Tile_Logic/E_TileType` (`self.getTileType` _array_element_2)
        (:`NewEnumerator5`
          (`KismetArrayLibrary.Array_Add` (`local.RandomizerPull`) "NewEnumerator5"))
        (:`NewEnumerator8`
          (`KismetArrayLibrary.Array_Add` (`local.RandomizerPull`) "NewEnumerator8"))))
    (bind _value (`self.getTile` _array_element))
    (set `/Game/Hex_Grid_Toolkit/Tile_Logic/BP_Tile.Type` _outitem _value)
    (`KismetSystemLibrary.PrintString` (`|GetEnumeratorNameAsString` _outitem) true true (struct :`G` 0.66 :`B` 1.0 :`A` 1.0) 4.0)
    (`KismetArrayLibrary.Array_Clear` (`local.RandomizerPull`))
    (`/Game/Hex_Grid_Toolkit/Tile_Logic/BP_Tile.FovUpdate` _value))
  (return))

(fn `findTilesOfType`
  (params (TileMap :type "Map of IntPoint Structure to /Game/Hex_Grid_Toolkit/Tile_Logic/BP_Tile Object Reference (by ref)") (Type :type "/Game/Hex_Grid_Toolkit/Tile_Logic/E_TileType Enum" :default "NewEnumerator0"))
  (returns (Shape :type "Array of IntPoint Structure"))
  (locals (ShapeLocal :type "Array of IntPoint Structure"))
  (bind _keys (`BlueprintMapLibrary.Map_Keys` TileMap))
  (for _array_element _keys
    (if (`|EnumEquality` (`/Game/Hex_Grid_Toolkit/Tile_Logic/BP_Tile.Type` (`BlueprintMapLibrary.Map_Find` TileMap _array_element)) Type)
      (`KismetArrayLibrary.Array_Add` (`local.ShapeLocal`) _array_element)))
  (return (`local.ShapeLocal`)))

(fn `getTile`
  (params (Axial :type "IntPoint Structure (by ref)"))
  (returns (Value :type "/Game/Hex_Grid_Toolkit/Tile_Logic/BP_Tile Object Reference"))
  (bind _value (`BlueprintMapLibrary.Map_Find` (`self.TileMap`) Axial))
  (`/Engine/EditorBlueprintResources/StandardMacros.IsValid` _value
    (:`Is Valid`
      (return _value))))

(fn `getTileType`
  (params (Axial :type "IntPoint Structure (by ref)"))
  (returns (Type :type "/Game/Hex_Grid_Toolkit/Tile_Logic/E_TileType Enum"))
  (bind _value (`BlueprintMapLibrary.Map_Find` (`self.TileMap`) Axial))
  (`/Engine/EditorBlueprintResources/StandardMacros.IsValid` _value
    (:`Is Valid`
      (return (`/Game/Hex_Grid_Toolkit/Tile_Logic/BP_Tile.Type` _value)))))

(fn `Hex_Logic_Definitions`
  (locals (Cube :type "IntVector Structure") (Axial :type "IntPoint Structure") (Offset :type "IntPoint Structure") (Polar :type "IntPoint Structure") (Location :type "Vector Structure") (Index :type Integer) (Steps :type Integer) (Degrees :type "Float (double-precision)") (Adjacent :type "/Game/Hex_Grid_Toolkit/Hex_Logic/E_Hex_Dir_Adjacent Enum") (Diagonal :type "/Game/Hex_Grid_Toolkit/Hex_Logic/E_Hex_Dir_Diagonal Enum") (Combined :type "/Game/Hex_Grid_Toolkit/Hex_Logic/E_Hex_Dir_Combined Enum") (Shape :type "Array of IntPoint Structure") (Path :type "Array of IntPoint Structure") (TileActorMap :type "Map of IntPoint Structure to /Game/Hex_Grid_Toolkit/Tile_Logic/BP_Tile Object Reference") (FlowMap :type "Map of IntPoint Structure to IntPoint Structure") (CostMap :type "Map of IntPoint Structure to Integer") (BP_Tile :type "/Game/Hex_Grid_Toolkit/Tile_Logic/BP_Tile Object Reference"))
  ;[1 0.6667 0] Dictionary of key concepts and naming conventions . To understand this toolkit.
)

(fn `RectangleSet`
  (params (FirstCord :type "IntPoint Structure") (SecoundCord :type "IntPoint Structure") (Type :type "/Game/Hex_Grid_Toolkit/Tile_Logic/E_TileType Enum" :default "NewEnumerator0"))
  (bind _path (`/Game/Hex_Grid_Toolkit/Hex_Logic/BPFL_Hex_Logic.getLine` FirstCord SecoundCord))
  (for _array_element _path
    (bind _value (`self.getTile` _array_element))
    (`/Engine/EditorBlueprintResources/StandardMacros.IsValid` _value
      (:`Is Valid`
        (set `/Game/Hex_Grid_Toolkit/Tile_Logic/BP_Tile.Type` Type _value)
        (`/Game/Hex_Grid_Toolkit/Tile_Logic/BP_Tile.Update` _value)))))

(fn `setTileSight`
  (params (Axial :type "Array of IntPoint Structure") (bSight :type Boolean))
  (for _array_element Axial
    (bind (_value _returnvalue) (`BlueprintMapLibrary.Map_Find` (`self.TileMap`) _array_element))
    (if _returnvalue
      (`/Game/Hex_Grid_Toolkit/Tile_Logic/BP_Tile.FovSet` _value bSight))))

(fn `Spawn Island`
  (params (Size :type Integer))
  (bind _shape (`/Game/Hex_Grid_Toolkit/Hex_Logic/BPFL_Hex_Logic.getHexagonShape` (struct) (- (`self.WorldSize`) (+ Size 4))))
  (bind _shape_2 (`/Game/Hex_Grid_Toolkit/Hex_Logic/BPFL_Hex_Logic.getHexagonShape` (`KismetArrayLibrary.Array_Random` _shape) Size))
  (for _array_element _shape_2
    (bind _value (`self.getTile` _array_element))
    (`/Engine/EditorBlueprintResources/StandardMacros.IsValid` _value
      (:`Is Valid`
        (set `/Game/Hex_Grid_Toolkit/Tile_Logic/BP_Tile.Type` "NewEnumerator5" _value)
        (`/Game/Hex_Grid_Toolkit/Tile_Logic/BP_Tile.FovUpdate` _value))))
  (return))

(fn `SpawnHills`
  (locals (`MakeHill?` :type Boolean :default true))
  (bind _shape (`self.findTilesOfType` (`self.TileMap`) "NewEnumerator5"))
  (for _array_element _shape
    (bind _shape_2 (`/Game/Hex_Grid_Toolkit/Hex_Logic/BPFL_Hex_Logic.getHexagonShape` _array_element 2))
    (for _array_element_2 _shape_2
      (if (not (and (not (`|EnumEquality` (`self.getTileType` _array_element_2) "NewEnumerator8")) (`.ReturnValue` (`BlueprintMapLibrary.Map_Find` (`self.TileMap`) _array_element_2))))
        (set `local.MakeHill?` false)))
    (if (`local.MakeHill?`)
      (bind _value (`self.getTile` _array_element_2))
      (set `/Game/Hex_Grid_Toolkit/Tile_Logic/BP_Tile.Type` "NewEnumerator0" _value)
      (`/Game/Hex_Grid_Toolkit/Tile_Logic/BP_Tile.Update` _value)
      (set `local.MakeHill?` true))))

(fn `spawnTile`
  (params (Axial :type "IntPoint Structure") (Type :type "/Game/Hex_Grid_Toolkit/Tile_Logic/E_TileType Enum" :default "NewEnumerator0"))
  (bind (_value _returnvalue) (`BlueprintMapLibrary.Map_Find` (`self.TileMap`) Axial))
  (`|ExecutionSequence`
    (:`then_0`
      ;[1 1 1] If actor exist at that axial, destroy it
      (if _returnvalue
        (`self.K2_DestroyActor` _value)))
    (:`then_1`
      (bind _returnvalue_2 (`|SpawnActorFromClass` "/Game/Hex_Grid_Toolkit/Tile_Logic/BP_Tile.BP_Tile_C" (`KismetMathLibrary.MakeTransform` (0.0 0.0 0.0)) "Undefined" "OverrideRootScale" null Axial Type null))
      (`BlueprintMapLibrary.Map_Add` (`self.TileMap`) Axial _returnvalue_2))))

(fn `UserConstructionScript`)

(fn `WorldGenerator`
  (locals (RandomizerPull :type "Array of /Game/Hex_Grid_Toolkit/Tile_Logic/E_TileType Enum"))
  (bind _shape (`/Game/Hex_Grid_Toolkit/Hex_Logic/BPFL_Hex_Logic.getHexagonShape` (struct) (`self.WorldSize`)))
  (for _array_element _shape
    (`self.spawnTile` _array_element "NewEnumerator8"))
  (`self.Spawn Island` 5)
  (`self.Spawn Island` 5)
  (`self.Spawn Island` 5)
  (`self.Spawn Island` 5)
  (`self.ClearLandmass`)
  (`/Game/System/RegionMenager.InitializeRegions` (`self.RegionMenager`) 5))