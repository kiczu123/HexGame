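; BP_Tile is a hex grid tile actor that places itself in the world from its axial coordinate.
; Its Type (Hills, Plains or Water) sets the mesh material color, dimmed when the tile is out of sight for fog of view.
; Region view swaps in the owning Region's color, falling back to the sight coloring otherwise.
; The construction script labels the tile with its axial coordinates.
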(event `self.ReceiveBeginPlay`
  (`self.Update`))

(event `Update`
  (bind (_location2d _location3d) (`/Game/Hex_Grid_Toolkit/Hex_Logic/BPFL_Hex_Logic.AxialToLocation` (`self.Axial`)))
  (`self.K2_SetActorTransform` (`KismetMathLibrary.MakeTransform` _location3d))
  (`self.FovUpdate`))

(event `FovSet`
  (params (OnSight :type Boolean))
  (set `self.OnSight` OnSight)
  (`self.FOVUpdate`))

(event `SetRegionView`
  (params (RegionView :type Boolean))
  (if (and RegionView (`KismetSystemLibrary.IsValid` (`self.Region`)))
    (`MeshComponent.SetVectorParameterValueOnMaterials` (`self.SM_Tile`) "Color" (`KismetMathLibrary.Conv_LinearColorToVector` (`/Game/System/Region.Color` (`self.Region`))))
    (else
      (`self.FovUpdate`))))

(event `FovUpdate`
  (bind _returnvalue (select `/Game/Hex_Grid_Toolkit/Tile_Logic/E_TileType` (`self.Type`) :`NewEnumerator0` (struct :`R` 0.109375 :`G` 0.103971 :`B` 0.097051 :`A` 1.0) :`NewEnumerator5` (struct :`R` 0.036249 :`G` 0.145833 :`B` 0.032348 :`A` 1.0) :`NewEnumerator8` (struct :`G` 0.102571 :`B` 0.895833 :`A` 1.0) :!type "LinearColor Structure"))
  (`MeshComponent.SetVectorParameterValueOnMaterials` (`self.SM_Tile`) "Color" (`KismetMathLibrary.Conv_LinearColorToVector` (select `bool` (`self.OnSight`) :`false` (* _returnvalue 0.35) :`true` _returnvalue))))

(fn `UserConstructionScript`
  (bind (_axial_x _axial_y) (break `IntPoint` (`self.Axial`)))
  (`TextRenderComponent.K2_SetText` (`self.TextRender`) (`KismetTextLibrary.Conv_StringToText` (`KismetStringLibrary.Concat_StrStr` "X:" (`KismetStringLibrary.Conv_IntToString` _axial_x) " Y:" (`KismetStringLibrary.Conv_IntToString` _axial_y)))))